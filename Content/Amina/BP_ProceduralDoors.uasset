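; Procedural door spawner that fills a square grid in the Y-Z plane with randomly chosen door actors on BeginPlay.
; A random stream seeded by GridSeed gives each cell a fixed chance of a door and picks one of three classes to spawn.
; Cell positions step from the root's location by width and height offsets.
; MatriceHeight sizes both axes, leaving MatriceWidth unused.
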(event `self.ReceiveBeginPlay`
  (bind _matriceheight (`self.MatriceHeight`))
  (bind (_relativelocation_x _relativelocation_y _relativelocation_z) (`KismetMathLibrary.BreakVector` (`SceneComponent.RelativeLocation` (`self.DefaultSceneRoot`))))
  (set `self.NewVar_0` (`self.K2_GetActorRotation` self))
  (set `self.Stream` (`KismetMathLibrary.MakeRandomStream` (`self.GridSeed`)))
  (for _index (range (`KismetMathLibrary.FTrunc` (* _matriceheight _matriceheight)))
    ;[0 0.3 0.7] Chancces for a door to be spawned
    (if (<= (`KismetMathLibrary.RandomFloatInRangeFromStream` 0.0 1.0 (`self.Stream`)) 0.3)
      (`self.SpawnDoor` (`KismetMathLibrary.MakeVector` _relativelocation_x (+ _relativelocation_y (* (`self.DoorOffsetWidth`) (`KismetMathLibrary.Conv_IntToDouble` (`KismetMathLibrary.FTrunc` (mod (`KismetMathLibrary.Conv_IntToDouble` _index) (`self.MatriceHeight`)))))) (+ _relativelocation_z (`self.MeshToSpawnSize`) (* (`self.DoorOffsetHeight`) (`KismetMathLibrary.Conv_IntToDouble` (`KismetMathLibrary.FTrunc` (/ (`KismetMathLibrary.Conv_IntToDouble` _index) (`self.MatriceHeight`))))))))
      (`self.K2_SetActorRotation` self (`self.NewVar_0`) false))))

(event `SpawnDoor`
  (params (Location :type "Vector Structure"))
  ;[0 0.3 0.7] Randomly spawn Door's children
  (switch `int` (`KismetMathLibrary.RandomIntegerInRangeFromStream` 1 3 (`self.Stream`))
    (:`1`
      (`|SpawnActorFromClass` "/Game/Amina/BP_ToSpawn1.BP_ToSpawn1_C" (`KismetMathLibrary.MakeTransform` Location) "Undefined" "OverrideRootScale" null null))
    (:`2`
      (`|SpawnActorFromClass` "/Game/Amina/BP_ToSpawn2.BP_ToSpawn2_C" (`KismetMathLibrary.MakeTransform` Location) "Undefined" "OverrideRootScale" null null))
    (:`3`
      (`|SpawnActorFromClass` "/Game/Amina/BP_ToSpawn3.BP_ToSpawn3_C" (`KismetMathLibrary.MakeTransform` Location) "Undefined" "OverrideRootScale" null null))))

(fn `UserConstructionScript`)